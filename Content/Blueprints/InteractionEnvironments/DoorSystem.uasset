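; A sliding door actor that opens when a Character overlaps its Enter trigger and closes when one overlaps its Exit trigger.
; An IsDoorOpen flag guards both events, so each plays its 2D sound and runs the OpenDoor timeline only on a change of state.
; The timeline drives two panels along local Z toward separate Zup and Zdown offsets, and closing plays it in reverse.
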(event OnComponentBeginOverlap(Enter)
  (params (OverlappedComponent :type Primitive%20Component%20Object%20Reference) (OtherActor :type Actor%20Object%20Reference) (OtherComp :type Primitive%20Component%20Object%20Reference) (OtherBodyIndex :type Integer) (bFromSweep :type Boolean) (SweepResult :type Hit%20Result%20Structure%20%28by%20ref%29))
  (Utilities|Casting|CastToCharacter OtherActor)
  (CallFunction|Opening))

(event OnComponentBeginOverlap(Exit)
  (params (OverlappedComponent :type Primitive%20Component%20Object%20Reference) (OtherActor :type Actor%20Object%20Reference) (OtherComp :type Primitive%20Component%20Object%20Reference) (OtherBodyIndex :type Integer) (bFromSweep :type Boolean) (SweepResult :type Hit%20Result%20Structure%20%28by%20ref%29))
  (Utilities|Casting|CastToCharacter OtherActor)
  (CallFunction|Closing))

(event Custom|Closing
  (if (Variables|Default|GetIsDoorOpen?)
    (Audio|PlaySound2D "/Game/Blueprints/Assets/Sounds/Close.Close" 1.0 1.0 0.0 0 0)
    (Variables|Default|SetIsDoorOpen? false)
    (bind _zoffset (Timeline|OpenDoor ReverseFromEnd)
      (:Update
        (Utilities|FlowControl|Sequence
          (:then_0
            (Transformation|SetRelativeLocation (Variables|Default|GetDoor1) (Math|Vector|MakeVector 0.0 0.0 (Math|Float|MapRangeClamped _zoffset 0.0 1.0 0.0 (Variables|Default|GetZup))) false false))
          (:then_1
            (Transformation|SetRelativeLocation (Variables|Default|GetDoor) (Math|Vector|MakeVector 0.0 0.0 (Math|Float|MapRangeClamped _zoffset 0.0 1.0 0.0 (Variables|Default|GetZdown))) false false)))))))

(event Custom|Opening
  (if (not (Variables|Default|GetIsDoorOpen?))
    (Audio|PlaySound2D "/Game/Blueprints/Assets/Sounds/Open.Open" 1.0 1.0 0.0 0 0)
    (Variables|Default|SetIsDoorOpen? true)
    (bind _zoffset (Timeline|OpenDoor PlayFromStart)
      (:Update
        (Utilities|FlowControl|Sequence
          (:then_0
            (Transformation|SetRelativeLocation (Variables|Default|GetDoor1) (Math|Vector|MakeVector 0.0 0.0 (Math|Float|MapRangeClamped _zoffset 0.0 1.0 0.0 (Variables|Default|GetZup))) false false))
          (:then_1
            (Transformation|SetRelativeLocation (Variables|Default|GetDoor) (Math|Vector|MakeVector 0.0 0.0 (Math|Float|MapRangeClamped _zoffset 0.0 1.0 0.0 (Variables|Default|GetZdown))) false false)))))))

(event EventBeginPlay)

(event Collision|EventActorBeginOverlap
  (params (OtherActor :type Actor%20Object%20Reference)))

(event EventTick
  (params (DeltaSeconds :type Float%20%28single-precision%29)))

(fn ConstructionScript)