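; Player character Blueprint with a configurable camera boom, sprint stamina, walk and aim states, and a stamina widget.
; Input sets movement flags and calls ChangeMovementState; sprint requires stamina and velocity aligned with actor forward.
; Tick drains stamina while sprinting in motion, otherwise regenerates it, and debug-prints CanSprint.
; Mouse-wheel macros zoom the boom with sounds, while keys trigger aimed firing, a death montage and camera shake.
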(event EventTick
  (params (DeltaSeconds :type Float%20%28single-precision%29))
  ;[0.3165 1 0.4845 1 40] StaminaSystem
  (Utilities|FlowControl|Sequence
    (:then_0
      (|StaminaSystem DeltaSeconds DeltaSeconds 2.0 8.0 (Variables|Character|GetMaxStamina) :!label _label))
    (:then_1
      (goto _label execute2))
    (:then_2
      (goto _label execute3))
    (:then_3
      (bind _output_get (Variables|Default|SetbCanSprint (Math|Vector|Equal(Vector) (Math|Vector|Normalize (Variables|/Script/Engine.MovementComponent|GetVelocity (Variables|Character|GetCharacterMovement))) (Transformation|GetActorForwardVector) 0.0001)))
      (Development|PrintString (Utilities|String|ToString(Boolean) _output_get) true true "(R=0.000000,G=0.660000,B=1.000000,A=1.000000)" 0.0))))

(event EventBeginPlay
  ;[0 1 0.2188 1 35] StaminaWidget
  (bind _returnvalue (UserInterface|CreateWidget "/Game/Blueprints/Widgets/StaminaWidget.StaminaWidget_C"))
  (bind _output_get (Variables|Default|SetStaminaWidget _returnvalue))
  (UserInterface|Viewport|AddtoViewport _output_get 0))

(event Input|ActionEvents|InputActionChangeWalk
  (params (Key :type Key%20Structure))
  (:Pressed
    (Variables|Default|SetWalkEnabled true)
    (Class|TPSCharacter|ChangeMovementState :!label _label))
  (:Released
    (Variables|Default|SetWalkEnabled false)
    (goto _label)))

(event Input|ActionEvents|InputActionChangeSprint
  (params (Key :type Key%20Structure))
  (:Pressed
    (Utilities|StaminaMacro
      (:Have%20Stamina
        (if (Variables|Default|GetbCanSprint)
          (Variables|Default|SetSprintRunEnabled true)
          (Class|TPSCharacter|ChangeMovementState :!label _label)))
      (:No%20Stamina
        (Variables|Default|SetSprintRunEnabled false :!label _label_2)
        (goto _label))))
  (:Released
    (goto _label_2)))

(event Input|KeyboardEvents|F
  (params (Key :type Key%20Structure))
  (:Pressed
    (CallFunction|CameraShakeEvent)))

(event Input|MouseEvents|RightMouseButton
  (params (Key :type Key%20Structure))
  (:Pressed
    (Variables|Default|SetAimEnabled true)
    (Class|TPSCharacter|ChangeMovementState :!label _label))
  (:Released
    (Variables|Default|SetAimEnabled false)
    (goto _label)))

(event Input|KeyboardEvents|SpaceBar
  (params (Key :type Key%20Structure))
  (:Pressed
    (if (Variables|Default|GetAimEnabled)
      (Animation|Montage|PlayMontage (Variables|Character|GetMesh) "/Game/Blueprints/Assets/Hero/Animation/Firing_Rifle_Montage.Firing_Rifle_Montage"))))

(event Input|KeyboardEvents|V
  (params (Key :type Key%20Structure))
  (:Pressed
    (Animation|Montage|PlayMontage (Variables|Character|GetMesh) "/Game/Blueprints/Assets/Hero/Animation/Death_Montage.Death_Montage")))

(event Input|MouseEvents|MouseWheelUp
  (params (Key :type Key%20Structure))
  ;[0.6014 0.2359 1 1 40] ZoomSystem
  (:Pressed
    (|ZoomIn 3e+02 3e+01 1e+01 :!label _label))
  (:Released
    (goto _label execute2)))

(event Input|MouseEvents|MouseWheelDown
  (params (Key :type Key%20Structure))
  ;[0.6014 0.2359 1 1 40] ZoomSystem
  (:Pressed
    (|ZoomOut 1.5e+03 3e+01 1e+01 :!label _label))
  (:Released
    (goto _label execute2)))

(fn ConstructionScript
  (Variables|/Script/Engine.SpringArmComponent|SetTargetArmLength (Variables|Default|GetCameraBoom) (Variables|Camera|GetHeight))
  (Transformation|SetRelativeRotation (Variables|Default|GetCameraBoom) (Variables|Camera|GetRotatorCamera) false false)
  (Variables|/Script/Engine.SpringArmComponent|SetbEnableCameraLag (Variables|Default|GetCameraBoom) (Variables|Camera|GetFlow))
  (Variables|/Script/Engine.SpringArmComponent|SetCameraLagSpeed (Variables|Default|GetCameraBoom) (Variables|Camera|GetCoefSmooth)))

(fn CameraShakeEvent
  (Camera|PlayWorldCameraShake "/Game/Blueprints/Game/BP_ShakeCamera.BP_ShakeCamera_C" (Transformation|GetWorldLocation (Variables|Default|GetTopDownCameraComponent)) 0.0 3e+01))